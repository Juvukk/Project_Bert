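; MenuPawn is a pawn, by its name for the menu, that gives its CineCamera a flickering glitch effect.
; Tick runs into a short Delay, which throttles updates to roughly ten per second.
; Each update rebuilds the camera's post-process settings with a random dirt mask texture from the Glitches array at high intensity, plus randomized black clip and film grain intensity.
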(event `self.ReceiveTick`
  (params (DeltaSeconds :type "Float (single-precision)"))
  (bind _glitches (`self.Glitches`))
  (`KismetSystemLibrary.Delay` 0.1)
  (set `CameraComponent.PostProcessSettings` (make `PostProcessSettings` :`FilmBlackClip` (`KismetMathLibrary.RandomFloatInRange` 0.5 1.0) :`BloomDirtMask` (`|GetArrayItem` _glitches (`KismetMathLibrary.RandomIntegerInRange` 0 (- (`KismetArrayLibrary.Array_Length` _glitches) 1))) :`BloomDirtMaskIntensity` 20.0 :`FilmGrainIntensity` (`KismetMathLibrary.RandomFloatInRange` 0.5 1.0)) (`self.CineCamera`)))

(fn `UserConstructionScript`)