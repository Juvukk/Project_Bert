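; BP_SecTouchPad is a security touchpad actor that shows one of three level-specific UI screens on its Widget component.
; On BeginPlay it picks a random SecLevel from three tiers, creates the matching WB_Level UI widget and assigns it to that component.
; It holds no other active logic, so any keypad interaction is not handled in this Blueprint's graphs.
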(event `self.ReceiveBeginPlay`
  (set `self.SecLevel` (`KismetMathLibrary.RandomIntegerInRange` 1 3))
  (if (== (`self.SecLevel`) 1)
    (bind _returnvalue (`|CreateWidget` "/Game/Assets/Keypad/WB_Level1UI.WB_Level1UI_C"))
    (`WidgetComponent.SetWidget` (`self.Widget`) _returnvalue)
    (elif (== (`self.SecLevel`) 2)
      (bind _returnvalue_2 (`|CreateWidget` "/Game/Assets/Keypad/WB_Level2UI.WB_Level2UI_C"))
      (`WidgetComponent.SetWidget` (`self.Widget`) _returnvalue_2)
      (elif (== (`self.SecLevel`) 3)
        (bind _returnvalue_3 (`|CreateWidget` "/Game/Assets/Keypad/WB_Level3UI.WB_Level3UI_C"))
        (`WidgetComponent.SetWidget` (`self.Widget`) _returnvalue_3)))))

(fn `UserConstructionScript`)