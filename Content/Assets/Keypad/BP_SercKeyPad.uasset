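; BP_SercKeyPad is a keypad actor that fires an unlock event after checking entered digits.
; On BeginPlay it binds to its Wb_KeypadBottom widget's CheckCode dispatcher.
; The check compares each EnteredCode element to itself, stepping a MultiGate whose fourth output calls Unlock, so the reject branch, which resets the gate, is effectively unreachable.
; GetCode fills Code with random digits but is never run, and the check ignores Code.
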(event `self.ReceiveBeginPlay`
  (bind _aswb_keypad_bottom (cast `/Game/Assets/Keypad/Wb_KeypadBottom` (`WidgetComponent.GetWidget` (`self.KeypadWidget`))))
  (bind _output_get (set `self.As Wb Keypad Bottom` _aswb_keypad_bottom))
  (add `/Game/Assets/Keypad/Wb_KeypadBottom.CheckCode` _output_get (delegate `CheckCode_Event`)))

(event `CheckCode_Event`
  (for (_array_element _array_index) (`/Game/Assets/Keypad/Wb_KeypadBottom.EnteredCode` (`self.As Wb Keypad Bottom`))
    (if (== _array_element (`|GetArrayItem` (`/Game/Assets/Keypad/Wb_KeypadBottom.EnteredCode` (`self.As Wb Keypad Bottom`)) _array_index))
      (`|MultiGate` false :!label _label
        (:`Out 3`
          (`self.UnlockEvent`)))
      (else
        (`KismetSystemLibrary.PrintString` "DoReject")
        (goto _label :!via `Reset`)))))

(fn `Get Code`
  (bind _returnvalue (`KismetMathLibrary.RandomIntegerInRange` 0 9))
  (for (_ _array_index) (`self.Code`)
    (`KismetSystemLibrary.PrintString` (`KismetStringLibrary.Conv_IntToString` _returnvalue))
    (`KismetArrayLibrary.Array_Set` (`self.Code`) _array_index _returnvalue)))

(fn `UserConstructionScript`)