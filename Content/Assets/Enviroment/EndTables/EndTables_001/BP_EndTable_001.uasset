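; End table actor with a sliding drawer and an item on top that gets knocked when the table is hit.
; A sphere trace at BeginPlay caches the static mesh above the base; base hits push it along the hitting actor's forward vector and wobble the root.
; Interaction triggers the child actor's spawn message and a dispatcher-driven timeline that slides the drawer to a limit, then disables its collision.
; IsInteractable always returns false.
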(event `self.ReceiveBeginPlay`
  (bind _returnvalue (`SceneComponent.K2_GetComponentLocation` (`self.Base`)))
  (bind _outhit (`KismetSystemLibrary.SphereTraceSingle` _returnvalue (+ _returnvalue (0.0 0.0 150.0)) 10.0 "TraceTypeQuery4"))
  (bind _asstatic_mesh_component (cast `StaticMeshComponent` (`.HitComponent` (`GameplayStatics.BreakHitResult` _outhit))))
  (set `self.BreakItemRef` _asstatic_mesh_component)
  (add `self.Open/CloseDrawer` (delegate `Open/CloseDrawer_Event`)))

(event `Open/CloseDrawer_Event`
  (bind _drawer (`self.Drawer`))
  (bind _relativelocation_x (`KismetMathLibrary.BreakVector` (`SceneComponent.RelativeLocation` _drawer)))
  (`KismetSystemLibrary.PrintString` "open")
  (bind (_direction _drawermovement) (`Timeline|Timeline`)
    (:`Update`
      (if (< _relativelocation_x 28.0)
        (`SceneComponent.K2_AddLocalOffset` _drawer (`KismetMathLibrary.MakeVector` _drawermovement) true false)
        (else
          (`PrimitiveComponent.SetCollisionResponseToAllChannels` (`self.Drawer`) "ECR_Ignore")
          (set `self.Tags` (`self.Tags_0`)))))))

(event `self.Base.OnComponentHit`
  (params (HitComponent :type "PrimitiveComponent Object Reference") (OtherActor :type "Actor Object Reference") (OtherComp :type "PrimitiveComponent Object Reference") (NormalImpulse :type "Vector Structure") (Hit :type "HitResult Structure (by ref)"))
  (bind _breakitemref (`self.BreakItemRef`))
  (bind _defaultsceneroot (`self.DefaultSceneRoot`))
  (bind (_relativerotation_roll _relativerotation_pitch _relativerotation_yaw) (`KismetMathLibrary.BreakRotator` (`SceneComponent.RelativeRotation` _defaultsceneroot)))
  (`/Engine/EditorBlueprintResources/StandardMacros.IsValid` _breakitemref
    (:`Is Valid`
      (`PrimitiveComponent.AddImpulse` _breakitemref (* (`self.GetActorForwardVector` OtherActor) (`self.PushForce`)) "None" false)
      (bind (_direction _wobbleamount) (`Timeline|wobble`)
        (:`Update`
          (`SceneComponent.K2_SetRelativeRotation` _defaultsceneroot (`KismetMathLibrary.MakeRotator` (+ _relativerotation_roll _wobbleamount) _relativerotation_pitch _relativerotation_yaw) false false))))))

(event `/Game/Assets/Interfaces/bpi_Interactable.OnInteract`
  (params (InteractingPlayer :type "/Game/Assets/Player/BP_FirstPersonCharacter Object Reference"))
  (message `/Game/Assets/Interfaces/Bpi_Spawn.OnSpawn` (`ChildActorComponent.ChildActor` (`self.ChildActor`)))
  (`self.Open/CloseDrawer_Event`))

(fn `IsInteractable`
  (returns (interactable :type Boolean))
  (return false))

(fn `UserConstructionScript`)