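; BP_Balloon is a balloon actor that reacts to being hit by launching upward.
; Capsule gravity switches on two seconds after play begins.
; A capsule hit prints a debug message, clears damping and gravity, and applies a fixed, mass-independent upward and sideways force to the static mesh.
; After a one-second delay, the capsule regains gravity and high linear damping to slow its movement.
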(event `self.ReceiveBeginPlay`
  (`self.SetLifeSpan` 0.0)
  (`KismetSystemLibrary.Delay` 2.0)
  (`PrimitiveComponent.SetEnableGravity` (`self.Capsule`) true))

(event `self.Capsule.OnComponentHit`
  (params (HitComponent :type "PrimitiveComponent Object Reference") (OtherActor :type "Actor Object Reference") (OtherComp :type "PrimitiveComponent Object Reference") (NormalImpulse :type "Vector Structure") (Hit :type "HitResult Structure (by ref)"))
  (`KismetSystemLibrary.PrintString` "fly")
  (`PrimitiveComponent.SetLinearDamping` (`self.Capsule`) 0.0)
  (`PrimitiveComponent.SetEnableGravity` (`self.Capsule`) false)
  (`PrimitiveComponent.AddForce` (`self.StaticMesh`) (-1000.0 -1000.0 5000.0) "None" true)
  (`KismetSystemLibrary.Delay` 1.0)
  (`PrimitiveComponent.SetLinearDamping` (`self.Capsule`) 10.0)
  (`PrimitiveComponent.SetEnableGravity` (`self.Capsule`) true))

(fn `UserConstructionScript`
  (`self.SetLifeSpan` 0.0))