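; Throwable paint can Blueprint that a player can grab, carry, charge and throw as a physics object.
; On interact, the player's Grabber grabs the Tin component, and Tick moves the grab target to the end point of the player's forward vector.
; Throw power builds in steps up to a cap, then throwing releases the tin with an impulse along the camera's forward direction.
; Cancel releases it without impulse, and IsInteractable always returns false.
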(event `/Game/Assets/Interfaces/bpi_Throw.DoThrow`
  (params (InteractingPlayer :type "/Game/Assets/Player/BP_FirstPersonCharacter Object Reference"))
  (set `self.isGrabbed` false)
  (`PhysicsHandleComponent.ReleaseComponent` (`/Game/Assets/Player/BP_FirstPersonCharacter.Grabber` InteractingPlayer))
  (`PrimitiveComponent.AddImpulse` (`self.Tin`) (* (`KismetMathLibrary.GetForwardVector` (`SceneComponent.K2_GetComponentRotation` (`/Game/Assets/Player/BP_FirstPersonCharacter.FirstPersonCamera` InteractingPlayer))) (`self.ThrowForce`)) "None" false)
  (set `self.ThrowForce` 0.0)
  (set `self.WasThrown` true))

(event `/Game/Assets/Interfaces/bpi_Throw.BuildThrowPower`
  (params (InteractingPlayer :type "/Game/Assets/Player/BP_FirstPersonCharacter Object Reference"))
  (if (< (`self.ThrowForce`) (`self.MaxThrowForce`))
    (set `self.ThrowForce` (+ (`self.ThrowForce`) 50.0))))

(event `/Game/Assets/Interfaces/Bpi_CancelInteract.OnCancel`
  (params (NewParam :type "/Game/Assets/Player/BP_FirstPersonCharacter Object Reference"))
  (set `self.isGrabbed` false)
  (`PhysicsHandleComponent.ReleaseComponent` (`/Game/Assets/Player/BP_FirstPersonCharacter.Grabber` NewParam)))

(event `/Game/Assets/Interfaces/bpi_Interactable.OnInteract`
  (params (InteractingPlayer :type "/Game/Assets/Player/BP_FirstPersonCharacter Object Reference"))
  (bind _tin (`self.Tin`))
  (bind _grabber (`/Game/Assets/Player/BP_FirstPersonCharacter.Grabber` InteractingPlayer))
  (set `self.Interacting Player` InteractingPlayer)
  (`KismetSystemLibrary.PrintString` (`KismetSystemLibrary.GetDisplayName` _grabber))
  (`PhysicsHandleComponent.GrabComponentAtLocation` _grabber _tin "None" (`SceneComponent.K2_GetComponentLocation` _tin))
  (`PrimitiveComponent.WakeRigidBody` (`self.Tin`) "None")
  (set `self.isGrabbed` true))

(event `self.ReceiveTick`
  (params (DeltaSeconds :type "Float (single-precision)"))
  (bind _interacting_player (`self.Interacting Player`))
  (if (`self.isGrabbed`)
    (bind (_start _end_) (`/Game/Assets/Player/BP_FirstPersonCharacter.ForwardVector` _interacting_player))
    (`PhysicsHandleComponent.SetTargetLocation` (`/Game/Assets/Player/BP_FirstPersonCharacter.Grabber` _interacting_player) _end_)))

(fn `IsInteractable`
  (returns (interactable :type Boolean))
  (return false))

(fn `UserConstructionScript`)