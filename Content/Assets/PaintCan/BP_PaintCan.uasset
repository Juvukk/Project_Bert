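; BP_PaintCan is a throwable paint can that impairs the sight of AI it hits.
; While WasThrown is set, Tick runs a debug-drawn sphere trace around the Tin component to detect a hit.
; The first valid hit clears the flag and activates Drops, then sends ReduceAISightMessage to actors tagged AI or prints a debug string for others.
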(event `self.ReceiveTick`
  (params (DeltaSeconds :type "Float (single-precision)"))
  (bind _returnvalue (`SceneComponent.K2_GetComponentLocation` (`self.Tin`)))
  (`parent.ReceiveTick` DeltaSeconds)
  (if (`self.WasThrown`)
    (bind _outhit (`KismetSystemLibrary.SphereTraceSingle` :`Start` _returnvalue :`End` _returnvalue :`Radius` 50.0 :`TraceChannel` "TraceTypeQuery1" :`bTraceComplex` true :`DrawDebugType` "Persistent"))
    (bind (_bblockinghit _binitialoverlap _time _distance _location _impactpoint _normal _impactnormal _physmat _hitactor) (`GameplayStatics.BreakHitResult` _outhit))
    (`/Engine/EditorBlueprintResources/StandardMacros.IsValid` _hitactor
      (:`Is Valid`
        (set `self.WasThrown` false)
        (`ActorComponent.Activate` (`self.Drops`) false)
        (if (`self.ActorHasTag` _hitactor "AI")
          (message `/Game/Assets/Interfaces/BPI_effectAI.ReduceAISight` _hitactor)
          (else
            (`KismetSystemLibrary.PrintString` "not AI ")))))))

(event `self.Tin.OnComponentHit`
  (params (HitComponent :type "PrimitiveComponent Object Reference") (OtherActor :type "Actor Object Reference") (OtherComp :type "PrimitiveComponent Object Reference") (NormalImpulse :type "Vector Structure") (Hit :type "HitResult Structure (by ref)")))

(fn `UserConstructionScript`
  (`parent.UserConstructionScript`))