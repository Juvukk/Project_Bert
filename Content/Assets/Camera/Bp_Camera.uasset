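; Security camera that sweeps at random rotation rates and reports a detected player's location to the MechaAI.
; On BeginPlay, a forward trace scales the CameraSensor volume by the distance from hit to trace end.
; A player overlapping the sensor fires the CamSee event, noted as triggering all cameras, which line-traces to confirm the player before alerting the AI.
; Tick re-randomizes rotation while Active and re-arms the camera after a delay otherwise.
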(event `self.ReceiveBeginPlay`
  (add `self.CamSee` (delegate `CamSee_Event`))
  (bind _outhit (`self.DoLineTrace`))
  (bind (_bblockinghit _binitialoverlap _time _distance _location _impactpoint _normal _impactnormal _physmat _hitactor _hitcomponent _hitbonename _bonename _hititem _elementindex _faceindex _tracestart _traceend) (`GameplayStatics.BreakHitResult` _outhit))
  (bind _returnvalue (/ (`KismetMathLibrary.VSize` (- _location _traceend)) 400.0))
  (`SceneComponent.SetWorldScale3D` (`self.CameraSensor`) (`KismetMathLibrary.MakeVector` _returnvalue _returnvalue _returnvalue)))

(event `CamSee_Event`
  (bind _returnvalue (`KismetMathLibrary.GetForwardVector` (`self.K2_GetActorRotation`)))
  ;[1 1 1] This Triggers all cameras not just the one who hit thw player
  (bind _start (`self.Forward` _returnvalue))
  (bind _outhit (`KismetSystemLibrary.LineTraceSingle` :`Start` _start :`End` (+ _returnvalue (`self.K2_GetActorLocation` (`self.Sweep Result Hit Actor`))) :`TraceChannel` "TraceTypeQuery1" :`bTraceComplex` true :`DrawDebugType` "Persistent"))
  (bind (_bblockinghit _binitialoverlap _time _distance _location _impactpoint _normal _impactnormal _physmat _hitactor) (`GameplayStatics.BreakHitResult` _outhit))
  (`/Engine/EditorBlueprintResources/StandardMacros.IsValid` _hitactor
    (:`Is Valid`
      (if (`self.ActorHasTag` _hitactor "Player")
        (message `/Game/Assets/Interfaces/bpi_Ai.CameraFoundActor` (`self.MechaAI`) _location false)
        (set `self.Active` false)
        (`KismetSystemLibrary.PrintString` "Cam Detected Player")
        (else
          (set `self.Active` true))))))

(event `self.CameraSensor.OnComponentBeginOverlap`
  (params (OverlappedComponent :type "PrimitiveComponent Object Reference") (OtherActor :type "Actor Object Reference") (OtherComp :type "PrimitiveComponent Object Reference") (OtherBodyIndex :type Integer) (bFromSweep :type Boolean) (SweepResult :type "HitResult Structure (by ref)"))
  (`/Engine/EditorBlueprintResources/StandardMacros.IsValid` OtherActor
    (:`Is Valid`
      (if (`self.ActorHasTag` OtherActor "Player")
        (set `self.Sweep Result Hit Actor` SweepResult_HitActor)
        (set `self.PlayerLoc` SweepResult_ImpactPoint)
        (set `self.Active` false)
        (`self.CamSee_Event`)))))

(event `self.ReceiveTick`
  (params (DeltaSeconds :type "Float (single-precision)"))
  (if (`self.Active`)
    (`KismetSystemLibrary.Delay` (`KismetMathLibrary.RandomFloatInRange` 0.25 (`self.Max`)))
    (`self.Rotation` (`self.Active`))
    (else
      (`KismetSystemLibrary.Delay` 2.5)
      (set `self.Active` true))))

(fn `DoLineTrace`
  (returns (OutHit :type "HitResult Structure"))
  (bind (_start _end) (`self.Forward` (`KismetMathLibrary.GetForwardVector` (`SceneComponent.K2_GetComponentRotation` (`self.DefaultSceneRoot`)))))
  (bind _outhit (`KismetSystemLibrary.LineTraceSingle` :`Start` _start :`End` _end :`TraceChannel` "TraceTypeQuery1" :`TraceColor` (struct :`R` 1.0 :`G` 1.0 :`B` 1.0 :`A` 1.0)))
  (return _outhit))

(fn `Forward`
  (params (EndForward :type "Vector Structure"))
  (returns (Start :type "Vector Structure") (End :type "Vector Structure"))
  (bind _returnvalue (`self.K2_GetActorLocation`))
  (return _returnvalue (+ _returnvalue (* EndForward (`self.InteractionDistance`)))))

(fn `Rotation`
  (params (Activate :type Boolean))
  (locals (OUT :type "Float (double-precision)" :default 0.0))
  (if Activate
    (set `local.OUT` (`KismetMathLibrary.RandomFloatInRange` -180.0 180.0))
    (else
      (set `local.OUT` 0.0)))
  (set `RotatingMovementComponent.RotationRate` (`KismetMathLibrary.MakeRotator` 0.0 0.0 (`local.OUT`)) (`self.RotatingMovement`))
  (return))

(fn `UserConstructionScript`)