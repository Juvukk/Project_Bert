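; A hide spot that conceals the player from the Mecha AI while they are inside its collision volume.
; Three seconds after the player enters, it marks them invisible to the AI and applies a vignette, without rechecking that they are still inside.
; At that moment, phone use also sets the AI's CowardsTimer to make the player easier to find.
; Leaving restores visibility and clears the post-process effect.
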(event `self.ReceiveBeginPlay`
  (bind _returnvalue (`GameplayStatics.GetActorOfClass` "/Game/Assets/GameManagement/PostProcessManager.PostProcessManager_C"))
  (set `self.PostProMan` _returnvalue)
  (bind _returnvalue_2 (`GameplayStatics.GetActorOfClass` "/Game/Assets/Mecha/Ai/Mecha_AI.Mecha_AI_C"))
  (set `self.MechaAI` _returnvalue_2)
  (bind _returnvalue_3 (`GameplayStatics.GetActorOfClass` "/Game/Assets/Player/BP_FirstPersonCharacter.BP_FirstPersonCharacter_C"))
  (set `self.Player` _returnvalue_3))

(event `self.InsideHideCol.OnComponentEndOverlap`
  (params (OverlappedComponent :type "PrimitiveComponent Object Reference") (OtherActor :type "Actor Object Reference") (OtherComp :type "PrimitiveComponent Object Reference") (OtherBodyIndex :type Integer))
  (`self.OnEndPlayerOverlap` OtherActor))

(event `OnEndPlayerOverlap`
  (params (OtherActor :type "Actor Object Reference"))
  (`/Engine/EditorBlueprintResources/StandardMacros.IsValid` OtherActor
    (:`Is Valid`
      (if (`self.ActorHasTag` OtherActor "Player")
        (set `self.PlayerInside` false)
        (`/Game/Assets/Mecha/Ai/Mecha_AI.SetPlayerVisible` (`self.MechaAI`) true)
        (message `/Game/Assets/Interfaces/BPI_PostProcessChange.ClearPostProcess` (`self.PostProMan`))))))

(event `self.InsideHideCol.OnComponentBeginOverlap`
  (params (OverlappedComponent :type "PrimitiveComponent Object Reference") (OtherActor :type "Actor Object Reference") (OtherComp :type "PrimitiveComponent Object Reference") (OtherBodyIndex :type Integer) (bFromSweep :type Boolean) (SweepResult :type "HitResult Structure (by ref)"))
  (`self.OnBeginPlayerOverlap` OtherActor))

(event `OnBeginPlayerOverlap`
  (params (OtherActor :type "Actor Object Reference"))
  (`/Engine/EditorBlueprintResources/StandardMacros.IsValid` OtherActor
    (:`Is Valid`
      (if (`self.ActorHasTag` OtherActor "Player")
        (set `self.PlayerInside` true)
        (`KismetSystemLibrary.Delay` 3.0)
        (`/Game/Assets/Mecha/Ai/Mecha_AI.SetPlayerVisible` (`self.MechaAI`) false)
        (`KismetSystemLibrary.PrintString` "Player Inside ")
        (message `/Game/Assets/Interfaces/BPI_PostProcessChange.ChangePostProcess` (`self.PostProMan`) (make `PostProcessSettings` :`VignetteIntensity` 0.8 :`DepthOfFieldVignetteSize` 400.0))
        ;[1 1 1] If you are hiding and using your phone you are easier to find
        (if (`/Game/Assets/Player/BP_FirstPersonCharacter.PhoneInUse` (`self.Player`))
          (set `/Game/Assets/Mecha/Ai/Mecha_AI.CowardsTimer` 5.0 (`self.MechaAI`)))))))

(fn `IsInteractable`
  (returns (interactable :type Boolean))
  (return false))

(fn `UserConstructionScript`)