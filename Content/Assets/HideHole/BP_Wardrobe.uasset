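; Wardrobe hiding spot with doors that open, close and break, controlling whether the mecha AI can see the player.
; Interaction alternates door sequences and passes the open state to MechaAI as player visibility; the player entering the inside collider does the same after a short delay.
; A hit swaps both doors once for spawned broken-door actors.
; IsInteractable returns false, and older timeline door logic is left unconnected.
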(event `/Game/Assets/Interfaces/bpi_Interactable.OnInteract`
  (params (InteractingPlayer :type "/Game/Assets/Player/BP_FirstPersonCharacter Object Reference") (objectInteracted :type "Actor Object Reference"))
  (if (== objectInteracted self)
    (`/Engine/EditorBlueprintResources/StandardMacros.FlipFlop`
      (:`A`
        (set `self.IsOpen` true)
        (`ActorSequenceComponent.PlaySequence` (`self.DoorOpen`)))
      (:`B`
        (set `self.IsOpen` false)
        (`ActorSequenceComponent.PlaySequence` (`self.DoorClose`))))
    (`/Game/Assets/Mecha/Ai/Mecha_AI.SetPlayerVisible` (`self.MechaAI`) (`self.IsOpen`))))

(event `/Game/Assets/Interfaces/BPI_BreakItem.BreakItem`
  (params (hitActor :type "Actor Object Reference"))
  (`/Engine/EditorBlueprintResources/StandardMacros.IsValid` hitActor
    (:`Is Valid`
      (if (== hitActor self)
        (if (not (`self.DoorsBroke`))
          (set `self.DoorsBroke` true)
          (`self.DoBreak` (`self.DoorR`))
          (`self.DoBreak` (`self.DoorL`)))))))

(event `self.InsideHideCol.OnComponentBeginOverlap`
  (params (OverlappedComponent :type "PrimitiveComponent Object Reference") (OtherActor :type "Actor Object Reference") (OtherComp :type "PrimitiveComponent Object Reference") (OtherBodyIndex :type Integer) (bFromSweep :type Boolean) (SweepResult :type "HitResult Structure (by ref)"))
  (`/Engine/EditorBlueprintResources/StandardMacros.IsValid` OtherActor
    (:`Is Valid`
      (if (`self.ActorHasTag` "Player")
        (`parent.OnBeginPlayerOverlap` OtherActor)
        (`KismetSystemLibrary.Delay` 3.0)
        (`/Game/Assets/Mecha/Ai/Mecha_AI.SetPlayerVisible` (`self.MechaAI`) (`self.IsOpen`))))))

(fn `DoBreak`
  (params (hitactor :type "StaticMeshComponent Object Reference"))
  ;[1 1 1] This Only Spawns Doors
  (`|SpawnActorFromClass` "/Game/Assets/HideHole/DoorsBroken/Bp_BrokenDoor.Bp_BrokenDoor_C" (`SceneComponent.K2_GetComponentToWorld` hitactor) "Undefined" "MultiplyWithRoot" null null)
  (`/Engine/EditorBlueprintResources/StandardMacros.IsValid` hitactor
    (:`Is Valid`
      (`ActorComponent.K2_DestroyComponent` hitactor))
    (:`Is Not Valid`
      (`KismetSystemLibrary.PrintString` "Do Break Not valid"))))

(fn `IsInteractable`
  (returns (interactable :type Boolean))
  (return false))

(fn `UserConstructionScript`)