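; BP_Vase is a noise item: a vase that shatters on hitting the floor and emits a noise event.
; A mesh hit handler requires sufficient speed, a Floor-tagged actor and an unset HasBroke flag before triggering NoiseEmmiter, skipping noise for AI-tagged actors.
; DoBreak spawns Bp_VaseBroke at the mesh's relative transform and destroys only the mesh component.
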(event `self.Item Mesh.OnComponentHit`
  (params (HitComponent :type "PrimitiveComponent Object Reference") (OtherActor :type "Actor Object Reference") (OtherComp :type "PrimitiveComponent Object Reference") (NormalImpulse :type "Vector Structure") (Hit :type "HitResult Structure (by ref)"))
  (set `self.Other Actor` OtherActor)
  (if (> (`KismetMathLibrary.VSize` (`SceneComponent.GetComponentVelocity` (`self.Item Mesh`))) 50.0)
    (if (`self.ActorHasTag` (`self.Other Actor`) "Floor")
      (if (not (`self.hasBroke`))
        (`KismetSystemLibrary.PrintString` "hit")
        (`/Engine/EditorBlueprintResources/StandardMacros.IsValid` (`self.Other Actor`)
          (:`Is Valid`
            (if (`self.ActorHasTag` (`self.Other Actor`) "AI")
              (`KismetSystemLibrary.PrintString` "Not player")
              (else
                (`/Game/Assets/NoiseItems/NoiseMaker.DoNoise_Event` (`self.NoiseEmmiter`) 5000.0)))
            (`self.DoBreak`))
          (:`Is Not Valid`
            (`KismetSystemLibrary.PrintString` "not valid")))))))

(fn `DoBreak`
  (`|SpawnActorFromClass` "/Game/Assets/NoiseItems/Vase/Broke/Bp_VaseBroke.Bp_VaseBroke_C" (`SceneComponent.GetRelativeTransform` (`self.Item Mesh`)) "Undefined" "MultiplyWithRoot" null null)
  (`/Engine/EditorBlueprintResources/StandardMacros.IsValid` (`self.Item Mesh`)
    (:`Is Valid`
      (`ActorComponent.K2_DestroyComponent` (`self.Item Mesh`)))))

(fn `UserConstructionScript`
  (`parent.UserConstructionScript`))