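; Stun gun bullet actor that shows a growing sphere with a short-lived light.
; Tick plays the Grow timeline, which scales the sphere by a multiplier.
; Timeline updates also start delays that switch off the point light, then destroy the actor.
; The overlap event has no effect: its tag check leads nowhere, and the logic swapping screen-tagged components to a glitch material on non-player actors is disconnected.
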(event `self.ReceiveBeginPlay`)

(event `self.ReceiveTick`
  (params (DeltaSeconds :type "Float (single-precision)"))
  (bind (_direction _scale) (`Timeline|Grow` :`NewTime` DeltaSeconds)
    (:`Update`
      (`SceneComponent.SetWorldScale3D` (`self.Sphere`) (`KismetMathLibrary.Conv_DoubleToVector` (* _scale (`self.ScaleMultiplier`))))
      (`KismetSystemLibrary.Delay` 0.2)
      (`SceneComponent.SetVisibility` (`self.PointLight`) false false)
      (`KismetSystemLibrary.Delay` 3.0)
      (`self.K2_DestroyActor`))))

(event `self.Sphere.OnComponentBeginOverlap`
  (params (OverlappedComponent :type "PrimitiveComponent Object Reference") (OtherActor :type "Actor Object Reference") (OtherComp :type "PrimitiveComponent Object Reference") (OtherBodyIndex :type Integer) (bFromSweep :type Boolean) (SweepResult :type "HitResult Structure (by ref)"))
  (if (`self.ActorHasTag` OtherActor "None")
    _))

(fn `UserConstructionScript`)