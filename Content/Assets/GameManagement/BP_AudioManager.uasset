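; BP_AudioManager is an audio manager Blueprint that optionally starts music on BeginPlay and exposes events for playing sounds in 2D or at a location.
; Random variants pick a clip through GetRandomSoundFromList, some adding random pitch or a delay.
; PlaySoundatLocationRandPitch does not randomize: it feeds MinPitch into volume, Volume into pitch and MaxPitch into start time.
; Two events retain debug "Hello" prints, and GetActorSoundParams is empty.
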(event `self.ReceiveBeginPlay`
  (if (`self.PlayMusic`)
    (`AudioComponent.Play` (`self.Audio_001`) 0.0)))

(event `/Game/Assets/Interfaces/BPI_Audio.PLay Sound Cue`
  (params (InCue :type "SoundCue Object Reference"))
  (`GameplayStatics.PlaySound2D` InCue 1.0 1.0 0.0 (`self.Concurrency Settings`) null false))

(event `/Game/Assets/Interfaces/BPI_Audio.PlaySoundAtLocationRandPitch`
  (params (Sound :type "SoundBase Object Reference") (Loc :type "Vector Structure") (`Min Pitch` :type "Float (double-precision)") (`Max Pitch` :type "Float (double-precision)") (Delay :type "Float (double-precision)") (Volume :type "Float (double-precision)"))
  (`KismetSystemLibrary.Delay` Delay)
  (`GameplayStatics.PlaySoundAtLocation` Sound Loc (struct) `Min Pitch` Volume `Max Pitch` null null null null))

(event `/Game/Assets/Interfaces/BPI_Audio.RandomPlayAudio`
  (params (SoundList :type "Array of SoundBase Object Reference (by ref)") (`IsUI?` :type Boolean))
  (bind _output (`self.GetRandomSoundFromList` SoundList))
  (`GameplayStatics.PlaySound2D` _output 1.0 1.0 0.0 null null))

(event `/Game/Assets/Interfaces/BPI_Audio.RandomPlayAudioRandomPitch`
  (params (SoundList :type "Array of SoundBase Object Reference (by ref)") (MinPitch :type "Float (double-precision)") (MaxPitch :type "Float (double-precision)") (`IsUI?` :type Boolean) (Owner :type "Actor Object Reference"))
  (`KismetSystemLibrary.PrintString` "Hello")
  (bind _output (`self.GetRandomSoundFromList` SoundList))
  (`GameplayStatics.PlaySound2D` _output 1.0 (`KismetMathLibrary.RandomFloatInRange` MinPitch MaxPitch) 0.0 null Owner `IsUI?`))

(event `/Game/Assets/Interfaces/BPI_Audio.PlayRandomSoundAtLocation`
  (params (SoundList :type "Array of SoundBase Object Reference (by ref)") (Loc :type "Vector Structure") (VolumeMultiplier :type "Float (double-precision)"))
  (`KismetSystemLibrary.PrintString` "Hello")
  (bind _output (`self.GetRandomSoundFromList` SoundList))
  (`GameplayStatics.PlaySoundAtLocation` _output Loc (struct) VolumeMultiplier 1.0 0.0 null null null null))

(event `/Game/Assets/Interfaces/BPI_Audio.PlayRandSoundAndPitchAtLoc`
  (params (SoundList :type "Array of SoundBase Object Reference (by ref)") (Loc :type "Vector Structure") (VolumeMultiplier :type "Float (double-precision)") (MinPitch :type "Float (double-precision)") (MaxPitch :type "Float (double-precision)") (Owner :type "Actor Object Reference") (Delay :type "Float (double-precision)"))
  (`KismetSystemLibrary.Delay` Delay)
  (bind _output (`self.GetRandomSoundFromList` SoundList))
  (`GameplayStatics.PlaySoundAtLocation` _output Loc (struct) VolumeMultiplier (`KismetMathLibrary.RandomFloatInRange` MinPitch MaxPitch) 0.0 null null Owner null))

(fn `GetActorSoundParams`
  (returns (Params :type "Array of AudioParameter Structure"))
  (return))

(fn `GetRandomSoundFromList`
  (params (Array :type "Array of SoundBase Object Reference"))
  (returns (Output :type "SoundBase Object Reference"))
  (return (`|GetArrayItem` Array (`KismetMathLibrary.RandomIntegerInRange` 0 (- (`KismetArrayLibrary.Array_Length` Array) 1)))))

(fn `UserConstructionScript`)