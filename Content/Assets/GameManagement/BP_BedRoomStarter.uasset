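; BP_BedRoomStarter is a one-shot trigger that allows the begin message when the player leaves the bedroom starter's box volume.
; On BeginPlay it caches the level's Bp_GameManager.
; The first end overlap by an actor tagged Player calls AllowBeginMessage on both Mecha and the game manager, then sets HasStarted to block repeats.
; Debug prints report the trigger and non-player exits.
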(event `self.ReceiveBeginPlay`
  (bind _returnvalue (`GameplayStatics.GetActorOfClass` "/Game/Assets/GameManagement/Bp_GameManager.Bp_GameManager_C"))
  (set `self.GameMan` _returnvalue))

(event `self.Box.OnComponentEndOverlap`
  (params (OverlappedComponent :type "PrimitiveComponent Object Reference") (OtherActor :type "Actor Object Reference") (OtherComp :type "PrimitiveComponent Object Reference") (OtherBodyIndex :type Integer))
  (if (`self.HasStarted`)
    _
    (elif (`self.ActorHasTag` OtherActor "Player")
      (`KismetSystemLibrary.PrintString` "Hello")
      (message `/Game/Assets/Interfaces/bpi_Ai.AllowBegin` (`self.Mecha`) true)
      (message `/Game/Assets/Interfaces/bpi_Ai.AllowBegin` (`self.GameMan`) true)
      (bind _output_get (set `self.HasStarted` true))
      (`KismetSystemLibrary.PrintString` (`KismetStringLibrary.Conv_BoolToString` _output_get))
      (else
        (`KismetSystemLibrary.PrintString` "This was not the player leaving")))))

(fn `UserConstructionScript`)