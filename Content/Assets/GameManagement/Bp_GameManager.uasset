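; Game manager that runs the opening input delay and the timed lockdown phase.
; On BeginPlay it disables input on the first player controller, then calls EnableInput after a short fixed delay.
; Once AllowBegin sets BeginGame, Tick counts LockDownTimer down.
; When the timer drops below zero, it latches LockDownEnded, prints a message and calls LockDownEnd once.
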(event `self.ReceiveBeginPlay`
  (bind _returnvalue (`GameplayStatics.GetPlayerController` 0))
  (`self.DisableInput` _returnvalue null)
  (`KismetSystemLibrary.Delay` 4.0)
  (`self.EnableInput` _returnvalue))

(event `self.ReceiveTick`
  (params (DeltaSeconds :type "Float (single-precision)"))
  (if (`self.BeginGame`)
    (if (not (`self.LockDownEnded`))
      (set `self.LockDownTimer` (- (`self.LockDownTimer`) DeltaSeconds))
      (if (< (`self.LockDownTimer`) 0.0)
        (`KismetSystemLibrary.PrintString` "lockdown Ended")
        (set `self.LockDownEnded` true)
        (`self.LockDownEnd`)))))

(event `/Game/Assets/Interfaces/bpi_Ai.AllowBegin`
  (params (`Yes Allow` :type Boolean))
  (set `self.BeginGame` `Yes Allow`))

(fn `UserConstructionScript`
  (`parent.UserConstructionScript`))