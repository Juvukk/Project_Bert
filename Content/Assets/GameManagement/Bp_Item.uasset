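; Bp_Item is an item actor that a player can pick up by interacting with it.
; When AllowPickUp is set, OnInteract prints a debug message and adds ItemCode to the interacting player's InventoryList if absent, then destroys the actor.
; An item whose code the player already holds stays in the world.
; IsInteractable always returns false, independent of AllowPickUp.
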(event `/Game/Assets/Interfaces/bpi_Interactable.OnInteract`
  (params (InteractingPlayer :type "/Game/Assets/Player/BP_FirstPersonCharacter Object Reference"))
  (bind _inventorylist (`/Game/Assets/Player/BP_FirstPersonCharacter.InventoryList` InteractingPlayer))
  (bind _itemcode (`self.ItemCode`))
  (if (`self.AllowPickUp`)
    (`KismetSystemLibrary.PrintString` "pick item")
    (if (not (`KismetArrayLibrary.Array_Contains` _inventorylist _itemcode))
      (`KismetArrayLibrary.Array_Add` _inventorylist _itemcode)
      (`self.K2_DestroyActor`))))

(fn `IsInteractable`
  (returns (interactable :type Boolean))
  (return false))

(fn `UserConstructionScript`)