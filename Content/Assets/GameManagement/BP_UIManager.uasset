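; Level UI manager that runs the loading screen, player HUD, end-game screen and quit-to-menu input.
; BeginPlay shows loading over a black camera fade, binds end-game and UI-fade events, then optionally creates the pointer and eye-open effect widgets.
; End game closes the eye, fades the camera, shows the end UI with a mouse cursor, then fades back in.
; A Timeline drives render opacity for widgets passed to the fade event.
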(event `self.ReceiveBeginPlay`
  (bind _returnvalue (`|CreateWidget` "/Game/Assets/UI/Loading.Loading_C" (`GameplayStatics.GetPlayerController` 0)))
  (`UserWidget.AddToViewport` _returnvalue 0)
  (`self.FadeCamera` 1.0 1.0 2.0)
  (`KismetSystemLibrary.Delay` 2.0)
  (`Widget.RemoveFromParent` _returnvalue)
  (add `self.EndGame` (delegate `EndGame_Event`))
  (add `self.FadeUI` (delegate `FadeUI_Event`))
  (if (`self.CreatePlayerPointer`)
    (bind _returnvalue_2 (`|CreateWidget` "/Game/Assets/UI/PlayerPointer.PlayerPointer_C" (`GameplayStatics.GetPlayerController` 0)))
    (set `self.PlayerPointer` _returnvalue_2)
    (`UserWidget.AddToViewport` _returnvalue_2 0)
    (bind _returnvalue_3 (`GameplayStatics.GetActorOfClass` "/Game/Assets/Player/Phone/BP_Phone.BP_Phone_C"))
    (bind _returnvalue_4 (`|CreateWidget` "/Game/Assets/UI/EyeEfftect.EyeEfftect_C" (`GameplayStatics.GetPlayerController` 0)))
    (`UserWidget.AddToViewport` _returnvalue_4 0)
    (bind _output_get (set `self.EyeEffect` _returnvalue_4))
    (`/Game/Assets/UI/EyeEfftect.EyeOpen` _output_get)))

(event `EndGame_Event`
  (bind _returnvalue (`GameplayStatics.GetPlayerController` 0))
  (`/Game/Assets/UI/EyeEfftect.EyeClose` (`self.EyeEffect`))
  (`self.FadeCamera` 0.0 1.0 1.5 (struct) false true)
  (`KismetSystemLibrary.Delay` 2.5)
  (bind _returnvalue_2 (`|CreateWidget` "/Game/Assets/UI/EndGameUi.EndGameUi_C" _returnvalue))
  (`UserWidget.AddToViewport` _returnvalue_2 0)
  (`WidgetBlueprintLibrary.SetInputMode_UIOnlyEx` _returnvalue _returnvalue_2 "DoNotLock" true)
  (set `PlayerController.bShowMouseCursor` true _returnvalue)
  (`self.FadeUI_Event` (`self.EyeEffect`))
  (`Widget.RemoveFromParent` (`self.EyeEffect`))
  (`self.FadeCamera` 1.0 0.0 1.0))

(event `FadeUI_Event` :!signature `self.FadeUI`
  (params (InWidget :type "UserWidget Object Reference"))
  (bind (_direction _opacity) (`Timeline|Timeline`)
    (:`Update`
      (`Widget.SetRenderOpacity` InWidget _opacity))))

(event `EnhancedInput|/Game/FirstPerson/Input/Actions/IA_QuitMenu`
  (params (ActionValue :type Boolean) (ElapsedSeconds :type "Float (double-precision)") (TriggeredSeconds :type "Float (double-precision)") (InputAction :type "InputAction Object Reference" :default "/Game/FirstPerson/Input/Actions/IA_QuitMenu.IA_QuitMenu"))
  (:`Triggered`
    (`GameplayStatics.OpenLevel` "StartMenu")))

(fn `FadeCamera`
  (params (FromAlpha :type "Float (single-precision)") (ToAlpha :type "Float (single-precision)") (Duration :type "Float (single-precision)") (Color :type "LinearColor Structure") (bShouldFadeAudio :type Boolean) (bHoldWhenFinished :type Boolean))
  (`PlayerCameraManager.StartCameraFade` (`GameplayStatics.GetPlayerCameraManager` 0) FromAlpha ToAlpha Duration Color bShouldFadeAudio bHoldWhenFinished))

(fn `UserConstructionScript`)