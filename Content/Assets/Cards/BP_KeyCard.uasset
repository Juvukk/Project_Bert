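; BP_KeyCard is an item Blueprint for a key card with a randomly chosen security level.
; On BeginPlay it picks one of three levels, then sets the matching card material on ItemMesh and the corresponding ItemID.
; Tick and OnInteract only forward to the parent class, and IsInteractable always returns false.
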(event `self.ReceiveBeginPlay`
  (`parent.ReceiveBeginPlay`)
  (bind _output_get (set `self.SecLevel` (`KismetMathLibrary.RandomIntegerInRange` 0 2)))
  (switch `int` _output_get
    (:`0`
      (`PrimitiveComponent.SetMaterial` (`self.Item Mesh`) 0 "/Game/Assets/Cards/Cardlevel1.Cardlevel1")
      (set `self.ItemID` "NewEnumerator0"))
    (:`1`
      (`PrimitiveComponent.SetMaterial` (`self.Item Mesh`) 0 "/Game/Assets/Cards/Cardlevel2.Cardlevel2")
      (set `self.ItemID` "NewEnumerator1"))
    (:`2`
      (`PrimitiveComponent.SetMaterial` (`self.Item Mesh`) 0 "/Game/Assets/Cards/Cardlevel3.Cardlevel3")
      (set `self.ItemID` "NewEnumerator2"))))

(event `self.ReceiveTick`
  (params (DeltaSeconds :type "Float (single-precision)"))
  (`parent.ReceiveTick` DeltaSeconds))

(event `/Game/Assets/Interfaces/bpi_Interactable.OnInteract`
  (params (InteractingPlayer :type "/Game/Assets/Player/BP_FirstPersonCharacter Object Reference"))
  (`parent.OnInteract` InteractingPlayer))

(fn `IsInteractable`
  (returns (interactable :type Boolean))
  (return false))

(fn `UserConstructionScript`
  (`parent.UserConstructionScript`))