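; BP_Phone is the player's phone actor, providing a toggleable torch and a keypad hacking tool.
; UseTorch flip-flops the SpotLight intensity between on and off.
; HackComplete? runs a sphere trace at the phone's location, with persistent debug drawing, and sends a hacked message with a phone reference to a hit actor tagged Keypad.
; GetHackedCode receives the keypad code, prints it and adds it to the phone's UI widget.
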(event `self.ReceiveBeginPlay`
  (bind _returnvalue (`GameplayStatics.GetActorOfClass` "/Game/Assets/Player/BP_FirstPersonCharacter.BP_FirstPersonCharacter_C"))
  (set `self.Player` _returnvalue))

(event `/Game/Assets/Interfaces/BPI_PhoneFunctions.UseTorch`
  (`/Engine/EditorBlueprintResources/StandardMacros.FlipFlop`
    (:`A`
      (set `self.LightIntensity` 100.0))
    (:`B`
      (set `self.LightIntensity` 0.0)))
  (`LightComponent.SetIntensity` (`self.SpotLight`) (`self.LightIntensity`)))

(event `/Game/Assets/Interfaces/BPI_KeyPadCodes.GetHackedCode`
  (params (getCodeFromKeypad :type String))
  (`KismetSystemLibrary.PrintString` (`KismetStringLibrary.Concat_StrStr` "Sned " getCodeFromKeypad))
  (message `/Game/Assets/Interfaces/BPI_KeyPadCodes.AddCodeToPhone` (`WidgetComponent.GetWidget` (`self.PhoneUIWId`)) getCodeFromKeypad))

(event `/Game/Assets/Interfaces/BPI_PhoneFunctions.HackComplete?`
  (params (`HackOpen?` :type Boolean))
  (bind _returnvalue (`self.K2_GetActorLocation`))
  (bind _outhit (`KismetSystemLibrary.SphereTraceSingle` :`Start` _returnvalue :`End` _returnvalue :`Radius` 100.0 :`TraceChannel` "TraceTypeQuery1" :`DrawDebugType` "Persistent"))
  (bind (_bblockinghit _binitialoverlap _time _distance _location _impactpoint _normal _impactnormal _physmat _hitactor) (`GameplayStatics.BreakHitResult` _outhit))
  (`/Engine/EditorBlueprintResources/StandardMacros.IsValid` _hitactor
    (:`Is Valid`
      (if (`self.ActorHasTag` _hitactor "Keypad")
        (message `/Game/Assets/Interfaces/BPI_KeyPadCodes.SendHacked` _hitactor self _hitactor)))))

(fn `UserConstructionScript`)