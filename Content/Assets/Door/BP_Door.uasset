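; Sliding door with an optional keypad lock and two signs whose material shows the locked state.
; A child BP_keyPad's unlock event clears the lock and opens it; interaction or non-player sphere overlap opens it only when unlocked.
; A timeline slides the mesh along Y, with a FlipFlop tracking IsOpen.
; Overlap exit, or a player entering while locked, fires a close dispatcher that reverses the timeline, bound only on doors without a keypad.
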(event `self.ReceiveBeginPlay`
  (bind _childactor (`ChildActorComponent.ChildActor` (`self.Child`)))
  (`/Engine/EditorBlueprintResources/StandardMacros.IsValid` _childactor
    (:`Is Valid`
      (bind _asbp_key_pad (cast `/Game/Assets/Door/Keypad/BP_keyPad` _childactor)
        (:`then`
          (add `/Game/Assets/Door/Keypad/BP_keyPad.Unlock` _asbp_key_pad (delegate `DoUnlock`)))
        (:`CastFailed`
          (`KismetSystemLibrary.PrintString` "faild"))))
    (:`Is Not Valid`
      (`KismetSystemLibrary.PrintString` (`KismetSystemLibrary.GetDisplayName` self))
      (add `self.CloseDoorEvent` (delegate `CloseDoorEvent_Event`)))))

(event `DoUnlock`
  (`self.SetDoorSigns` 1)
  (set `self.IsLocked` false)
  (if (not (`self.IsLocked`)) :!label _label
    (bind (_direction _delta) (`Timeline|OpenDoor_` :!label _label_2)
      (:`Update`
        (`self.MoveDoor` _delta 141.0))
      (:`Finished`
        (`/Engine/EditorBlueprintResources/StandardMacros.FlipFlop`
          (:`A`
            (set `self.IsOpen` true))
          (:`B`
            (set `self.IsOpen` false)))))))

(event `CloseDoorEvent_Event`
  (if (`self.IsOpen`)
    (goto _label_2 :!via `Reverse`)))

(event `/Game/Assets/Interfaces/bpi_OpenDoor.DoOpenDoor`
  (goto _label))

(event `self.OnInteract`
  (params (InteractingPlayer :type "/Game/Assets/Player/BP_FirstPersonCharacter Object Reference"))
  (set `self.Other Actor` InteractingPlayer)
  (`/Game/Assets/Interfaces/bpi_OpenDoor.DoOpenDoor`))

(event `self.Sphere.OnComponentBeginOverlap`
  (params (OverlappedComponent :type "PrimitiveComponent Object Reference") (OtherActor :type "Actor Object Reference") (OtherComp :type "PrimitiveComponent Object Reference") (OtherBodyIndex :type Integer) (bFromSweep :type Boolean) (SweepResult :type "HitResult Structure (by ref)"))
  (`|ExecutionSequence`
    (:`then_0`
      (`/Engine/EditorBlueprintResources/StandardMacros.IsValid` OtherActor
        (:`Is Valid`
          (if (`self.ActorHasTag` OtherActor "Player")
            (if (`self.IsLocked`)
              (`self.CloseDoorEvent_Event`))
            (else
              ;[1 1 1] If it's not the player it must be the mecha
              (`self.DoOpenDoor`))))))
    (:`then_1`
      (if (`self.IsLocked`)
        (`self.SetDoorSigns` 0)
        (else
          (set `self.Tags` (`self.UnlockedTags`))
          (`self.SetDoorSigns` 1))))))

(event `self.Sphere.OnComponentEndOverlap`
  (params (OverlappedComponent :type "PrimitiveComponent Object Reference") (OtherActor :type "Actor Object Reference") (OtherComp :type "PrimitiveComponent Object Reference") (OtherBodyIndex :type Integer))
  (`/Engine/EditorBlueprintResources/StandardMacros.IsValid` OtherActor
    (:`Is Valid`
      (`self.CloseDoorEvent_Event`))))

(fn `IsInteractable`
  (returns (interactable :type Boolean))
  (return false))

(fn `MoveDoor`
  (params (A :type "Float (double-precision)") (B :type "Float (double-precision)"))
  (`SceneComponent.K2_SetRelativeLocation` (`self.Door`) (`KismetMathLibrary.MakeVector` 0.0 (* A B)) true false))

(fn `MoveSpotLightToPlayer`
  (params (Target :type "Actor Object Reference")))

(fn `NewFunction`)

(fn `SetDoorSigns`
  (params (MaterialIndex :type Integer))
  (bind _output (`|GetArrayItem` (`self.SignMaterials`) MaterialIndex))
  (`PrimitiveComponent.SetMaterial` (`self.Sign 1`) 0 _output)
  (`PrimitiveComponent.SetMaterial` (`self.Sign 2`) 0 _output))

(fn `UserConstructionScript`)