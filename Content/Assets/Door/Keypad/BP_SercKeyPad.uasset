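; Keypad actor for a door that checks a player-entered code and fires an unlock event when it matches.
; On BeginPlay it registers with the game manager and binds to its keypad widget's check-code event.
; The check compares digits against a code set via SendCode or randomized by GetCode, using a MultiGate to count matches to four.
; Success or mismatch shows a widget message and plays a sound, and a mismatch resets the gate.
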(event `self.ReceiveBeginPlay`
  (bind _returnvalue (`GameplayStatics.GetActorOfClass` "/Game/Assets/GameManagement/Bp_GameManager.Bp_GameManager_C"))
  (`KismetArrayLibrary.Array_AddUnique` (`/Game/Assets/GameManagement/Bp_GameManager.Keypads` _returnvalue) self)
  (bind _aswb_keypad_bottom (cast `/Game/Assets/Door/Keypad/Wb_KeypadBottom` (`WidgetComponent.GetWidget` (`self.KeypadWidget`))))
  (bind _output_get (set `self.As Wb Keypad Bottom` _aswb_keypad_bottom))
  (add `/Game/Assets/Door/Keypad/Wb_KeypadBottom.CheckCode` _output_get (delegate `CheckCode_Event`)))

(event `CheckCode_Event`
  (for (_array_element _array_index) (`self.Code`)
    (if (== _array_element (`|GetArrayItem` (`/Game/Assets/Door/Keypad/Wb_KeypadBottom.EnteredCode` (`self.As Wb Keypad Bottom`)) _array_index))
      (`|MultiGate` false :!label _label
        (:`Out 3`
          (message `/Game/Assets/Interfaces/Bpi_UI.KeyPad_Accept` (`self.As Wb Keypad Bottom`))
          (`self.UnlockEvent`)
          (`GameplayStatics.PlaySound2D` "/Game/Assets/Audio/Keypad/Keypad_Correct.Keypad_Correct" 10.0 1.0 0.0 "/Game/Assets/Audio/Keypad/Keypad.Keypad" null)))
      (else
        (message `/Game/Assets/Interfaces/Bpi_UI.Keypad_Reject` (`self.As Wb Keypad Bottom`))
        (`GameplayStatics.PlaySound2D` "/Game/Assets/Audio/Keypad/Keypad_Reject.Keypad_Reject" 10.0 1.0 0.0 "/Game/Assets/Audio/Keypad/Keypad.Keypad" null)
        (goto _label :!via `Reset`)))))

(event `/Game/Assets/Interfaces/BPI_KeyPadCodes.SendCode`
  (params (FromKeyPad :type "Array of Integer (by ref)"))
  (set `self.Code` FromKeyPad))

(fn `Get Code`
  (bind _returnvalue (`KismetMathLibrary.RandomIntegerInRange` 0 9))
  (for (_ _array_index) (`self.Code`)
    (`KismetSystemLibrary.PrintString` (`KismetStringLibrary.Conv_IntToString` _returnvalue))
    (`KismetArrayLibrary.Array_Set` (`self.Code`) _array_index _returnvalue)))

(fn `UserConstructionScript`)