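; BP_SecTouchPad is an interactable security keypad that rolls a random clearance level from 1 to 3 at BeginPlay.
; It shows the matching level widget on its widget component.
; On interact, the player's held item is read as an integer: values from the pad's level up to 3 call Unlock, others call the Reject event.
; Rejection reaches the active widget through chained per-level validity-check macros.
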(event `self.ReceiveBeginPlay`
  (`self.GetRandomSecLevel`)
  (`self.SetUI`)
  (add `self.RejectEvent` (delegate `DoReject`)))

(event `DoReject`
  (bind _level1 (`self.Level1`))
  (bind _level2 (`self.Level2`))
  (bind _level3 (`self.Level3`))
  (`/Engine/EditorBlueprintResources/StandardMacros.IsValid` _level1
    (:`Is Valid`
      (`/Game/Assets/Door/Keypad/WB_Level1UI.Reject` _level1))
    (:`Is Not Valid`
      (`KismetSystemLibrary.PrintString` "Level 1 not valid")
      (`/Engine/EditorBlueprintResources/StandardMacros.IsValid` _level2
        (:`Is Valid`
          (`/Game/Assets/Door/Keypad/WB_Level2UI.Reject` _level2)
          (`/Engine/EditorBlueprintResources/StandardMacros.IsValid` _level3
            (:`Is Valid`
              (`/Game/Assets/Door/Keypad/WB_Level3UI.reject` _level3))))))))

(event `/Game/Assets/Interfaces/bpi_Interactable.OnInteract`
  (params (InteractingPlayer :type "/Game/Assets/Player/BP_FirstPersonCharacter Object Reference") (objectInteracted :type "Actor Object Reference"))
  (bind _returnvalue (`KismetMathLibrary.Conv_ByteToInt` (`/Game/Assets/Player/BP_FirstPersonCharacter.HeldItem` InteractingPlayer)))
  (if (<= _returnvalue 3)
    (if (>= _returnvalue (`self.KeyPadSecLevel`))
      (`self.Unlock`)
      (else
        (`KismetSystemLibrary.PrintString` "Call reject" :!label _label)
        (`self.RejectEvent`)))
    (else
      (goto _label))))

(fn `GetRandomSecLevel`
  (set `self.KeyPadSecLevel` (`KismetMathLibrary.RandomIntegerInRange` 1 3)))

(fn `IsInteractable`
  (returns (interactable :type Boolean))
  (return false))

(fn `SetUI`
  (if (== (`self.KeyPadSecLevel`) 1)
    (bind _returnvalue (`|CreateWidget` "/Game/Assets/Door/Keypad/WB_Level1UI.WB_Level1UI_C"))
    (bind _output_get (set `self.Level1` _returnvalue))
    (`WidgetComponent.SetWidget` (`self.Widget`) _output_get)
    (elif (== (`self.KeyPadSecLevel`) 2)
      (bind _returnvalue_2 (`|CreateWidget` "/Game/Assets/Door/Keypad/WB_Level2UI.WB_Level2UI_C"))
      (bind _output_get_2 (set `self.Level2` _returnvalue_2))
      (`WidgetComponent.SetWidget` (`self.Widget`) _output_get_2)
      (elif (== (`self.KeyPadSecLevel`) 3)
        (bind _returnvalue_3 (`|CreateWidget` "/Game/Assets/Door/Keypad/WB_Level3UI.WB_Level3UI_C"))
        (bind _output_get_3 (set `self.Level3` _returnvalue_3))
        (`WidgetComponent.SetWidget` (`self.Widget`) _output_get_3)))))

(fn `UserConstructionScript`)