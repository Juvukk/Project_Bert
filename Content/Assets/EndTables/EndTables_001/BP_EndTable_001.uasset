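; End table prop with a drawer that yields a random card and a wobble that knocks the item resting on it.
; On BeginPlay it picks a card class and sphere-traces upward from the base to cache that item's mesh.
; Hits on the base push the cached mesh along the hitting actor's forward vector and play the wobble timeline.
; OnInteract spawns the card and slides the drawer open with it, though IsInteractable returns false.
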(event `self.ReceiveBeginPlay`
  (bind _returnvalue (`SceneComponent.K2_GetComponentLocation` (`self.Base`)))
  (bind _outhit (`KismetSystemLibrary.SphereTraceSingle` :`Start` _returnvalue :`End` (+ _returnvalue (0.0 0.0 150.0)) :`Radius` 10.0 :`TraceChannel` "TraceTypeQuery4" :`DrawDebugType` "Persistent"))
  (bind _asstatic_mesh_component (cast `StaticMeshComponent` (`.HitComponent` (`GameplayStatics.BreakHitResult` _outhit))))
  (set `self.BreakItemRef` _asstatic_mesh_component)
  (set `self.ClassIndex` (`KismetMathLibrary.RandomIntegerInRange` 0 (- (`KismetArrayLibrary.Array_Length` (`self.RandomCard`)) 1))))

(event `self.Base.OnComponentHit`
  (params (HitComponent :type "PrimitiveComponent Object Reference") (OtherActor :type "Actor Object Reference") (OtherComp :type "PrimitiveComponent Object Reference") (NormalImpulse :type "Vector Structure") (Hit :type "HitResult Structure (by ref)"))
  (bind _breakitemref (`self.BreakItemRef`))
  (bind _defaultsceneroot (`self.DefaultSceneRoot`))
  (bind (_relativerotation_roll _relativerotation_pitch _relativerotation_yaw) (`KismetMathLibrary.BreakRotator` (`SceneComponent.RelativeRotation` _defaultsceneroot)))
  (`/Engine/EditorBlueprintResources/StandardMacros.IsValid` _breakitemref
    (:`Is Valid`
      (`PrimitiveComponent.AddImpulse` _breakitemref (* (`self.GetActorForwardVector` OtherActor) (`self.PushForce`)) "None" false)
      (bind (_direction _wobbleamount) (`Timeline|wobble`)
        (:`Update`
          (`SceneComponent.K2_SetRelativeRotation` _defaultsceneroot (`KismetMathLibrary.MakeRotator` (+ _relativerotation_roll _wobbleamount) _relativerotation_pitch _relativerotation_yaw) false false))))))

(event `/Game/Assets/Interfaces/bpi_Interactable.OnInteract`
  (params (InteractingPlayer :type "/Game/Assets/Player/BP_FirstPersonCharacter Object Reference"))
  (bind _drawer (`self.Drawer`))
  (bind _relativelocation_x (`KismetMathLibrary.BreakVector` (`SceneComponent.RelativeLocation` _drawer)))
  (bind _returnvalue (`|SpawnActorFromClass` (`|GetArrayItem` (`self.RandomCard`) (`self.ClassIndex`)) (`SceneComponent.GetRelativeTransform` (`self.SpawnPoint`)) "Undefined" "MultiplyWithRoot" null null))
  (bind (_direction _opendrawer) (`Timeline|DrawerOpen`)
    (:`Update`
      (if (< _relativelocation_x 28.0)
        (`SceneComponent.K2_AddLocalOffset` _drawer _opendrawer false false)
        (`self.K2_SetActorLocation` _returnvalue (`SceneComponent.K2_GetComponentLocation` (`self.Drawer`)) false true)))))

(fn `IsInteractable`
  (returns (interactable :type Boolean))
  (return false))

(fn `UserConstructionScript`)