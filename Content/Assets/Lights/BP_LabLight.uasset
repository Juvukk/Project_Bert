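; BP_LabLight is a switchable lab light that shows or hides a SpotLight.
; It overrides the parent's SwitchLights event and responds only when LightToSwitch is itself.
; It sets SpotLight visibility from LightIsON without propagating to children, then calls the parent SwitchLights with ISLightON fixed to false.
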(event `self.SwitchLights`
  (params (LightToSwitch :type "/Game/Assets/Lights/BP_LightRound Object Reference") (`ISLightON?` :type Boolean))
  (if (== LightToSwitch self)
    (`SceneComponent.SetVisibility` (`self.SpotLight`) (`self.LightIsON`) false)
    (`parent.SwitchLights` self false)))

(fn `UserConstructionScript`
  (`parent.UserConstructionScript`))