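; BP_LightNOMesh is a light actor that shows or hides its PointLight according to the LightIsON flag.
; TurnLights applies the flag to the light's visibility on BeginPlay and whenever SwitchLights names this actor as its target.
; TurnLights only reads LightIsON, and nothing in these graphs changes its value.
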(event `self.ReceiveBeginPlay`
  (`parent.ReceiveBeginPlay`)
  (`self.TurnLights`))

(event `self.SwitchLights`
  (params (LightToSwitch :type "/Game/Assets/Lights/BP_LightRound Object Reference") (`ISLightON?` :type Boolean))
  (if (== LightToSwitch self)
    (`self.TurnLights`)))

(fn `TurnLights`
  (`SceneComponent.SetVisibility` (`self.PointLight`) (`self.LightIsON`) false))

(fn `UserConstructionScript`
  (`parent.UserConstructionScript`))