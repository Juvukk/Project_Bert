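; Round point light actor that intermittently toggles itself on and off like a malfunctioning fixture.
; A Delay on Tick paces a random, high-probability toggle every few seconds through TurnLights, which sets visibility to the inverse of its input.
; Switching on randomly plays a malfunction sound at varied pitch and volume through BP_AudioManager.
; BeginPlay and a SwitchLights event targeting this actor both force the light on.
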(event `self.ReceiveBeginPlay`
  (`parent.ReceiveBeginPlay`)
  (`self.TurnLights` false)
  (bind _returnvalue (`GameplayStatics.GetActorOfClass` "/Game/Assets/GameManagement/BP_AudioManager.BP_AudioManager_C"))
  (set `self.AudioMan` _returnvalue))

(event `self.ReceiveTick`
  (params (DeltaSeconds :type "Float (single-precision)"))
  (`parent.ReceiveTick` DeltaSeconds)
  (`KismetSystemLibrary.Delay` 7.25)
  (if (>= (`KismetMathLibrary.RandomIntegerInRange` 0 4) 1)
    (`self.TurnLights` (`self.IsON`))))

(event `self.SwitchLights`
  (params (LightToSwitch :type "/Game/Assets/Lights/BP_LightRound Object Reference"))
  (if (== LightToSwitch self)
    (`self.TurnLights` false)))

(fn `TurnLights`
  (params (`ON?` :type Boolean))
  (bind _output_get (set `self.IsON` (not `ON?`)))
  (`SceneComponent.SetVisibility` (`self.PointLight`) _output_get false)
  (if (`KismetMathLibrary.RandomBool`)
    (if _output_get
      (message `/Game/Assets/Interfaces/BPI_Audio.PlaySoundAtLocationRandPitch` (`self.AudioMan`) "/Game/Assets/Audio/SFX/LightMalfunction.LightMalfunction" (`self.K2_GetActorLocation`) -10.0 5.0 0.0 (`KismetMathLibrary.Conv_IntToDouble` (`KismetMathLibrary.RandomIntegerInRange` 1 10))))))

(fn `UserConstructionScript`
  (`parent.UserConstructionScript`))