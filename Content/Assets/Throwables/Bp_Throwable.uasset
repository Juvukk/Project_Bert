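; Throwable physics prop that a player picks up, carries, charges and throws.
; OnInteract grabs the mesh with the player's Grabber, and Tick holds it at the endpoint supplied by the player's ForwardVector with zeroed rotation.
; BuildThrowPower raises force toward a cap, then DoThrow releases the mesh with an impulse along camera forward.
; BeginPlay caches a child NoiseMaker, unused here, and IsInteractable returns false.
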(event `/Game/Assets/Interfaces/bpi_Throw.DoThrow`
  (params (InteractingPlayer :type "/Game/Assets/Player/BP_FirstPersonCharacter Object Reference"))
  (bind (_returnvalue_x _returnvalue_y _returnvalue_z) (`KismetMathLibrary.BreakVector` (* (`KismetMathLibrary.GetForwardVector` (`PlayerCameraManager.GetCameraRotation` (`GameplayStatics.GetPlayerCameraManager` 0))) (`self.ThrowForce`))))
  (set `self.isGrabbed` false)
  (`PhysicsHandleComponent.ReleaseComponent` (`/Game/Assets/Player/BP_FirstPersonCharacter.Grabber` InteractingPlayer))
  (`PrimitiveComponent.AddImpulse` (`self.StaticMesh`) (`KismetMathLibrary.MakeVector` _returnvalue_x _returnvalue_y _returnvalue_z) "None" false)
  (set `self.ThrowForce` 0.0)
  (set `self.WasThrown` true)
  (`KismetSystemLibrary.PrintString` "weee"))

(event `/Game/Assets/Interfaces/Bpi_CancelInteract.OnCancel`
  (params (NewParam :type "/Game/Assets/Player/BP_FirstPersonCharacter Object Reference"))
  (set `self.isGrabbed` false)
  (`PhysicsHandleComponent.ReleaseComponent` (`/Game/Assets/Player/BP_FirstPersonCharacter.Grabber` NewParam)))

(event `/Game/Assets/Interfaces/bpi_Throw.BuildThrowPower`
  (params (InteractingPlayer :type "/Game/Assets/Player/BP_FirstPersonCharacter Object Reference"))
  (if (< (`self.ThrowForce`) (`self.MaxThrowForce`))
    (bind _output_get (set `self.ThrowForce` (+ (`self.ThrowForce`) (`self.AddToThrowForce`))))
    (`KismetSystemLibrary.PrintString` (`KismetStringLibrary.Conv_DoubleToString` _output_get))))

(event `/Game/Assets/Interfaces/bpi_Interactable.OnInteract`
  (params (InteractingPlayer :type "/Game/Assets/Player/BP_FirstPersonCharacter Object Reference"))
  (bind _staticmesh (`self.StaticMesh`))
  (bind _grabber (`/Game/Assets/Player/BP_FirstPersonCharacter.Grabber` InteractingPlayer))
  ;[1 1 1] We wont need this in the new inventory system
  (set `self.Interacting Player` InteractingPlayer)
  (`KismetSystemLibrary.PrintString` (`KismetSystemLibrary.GetDisplayName` _grabber))
  (`PhysicsHandleComponent.GrabComponentAtLocation` _grabber _staticmesh "None" (`SceneComponent.K2_GetComponentLocation` _staticmesh))
  (`PrimitiveComponent.WakeRigidBody` (`self.StaticMesh`) "None")
  (set `self.isGrabbed` true))

(event `self.ReceiveTick`
  (params (DeltaSeconds :type "Float (single-precision)"))
  (bind _interacting_player (`self.Interacting Player`))
  (bind _grabber (`/Game/Assets/Player/BP_FirstPersonCharacter.Grabber` _interacting_player))
  (if (`self.isGrabbed`)
    (bind (_start _end_) (`/Game/Assets/Player/BP_FirstPersonCharacter.ForwardVector` _interacting_player))
    (`PhysicsHandleComponent.SetTargetLocation` _grabber _end_)
    (`PhysicsHandleComponent.SetTargetRotation` :`self` _grabber)))

(event `self.ReceiveBeginPlay`
  (bind _asnoise_maker (cast `/Game/Assets/NoiseItems/NoiseMaker` (`ChildActorComponent.ChildActor` (`self.NoiseMaker`))))
  (set `self.NoiseEmmiter` _asnoise_maker))

(fn `IsInteractable`
  (returns (interactable :type Boolean))
  (return false))

(fn `UserConstructionScript`)